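; Post-process manager actor that shows a post-process effect at the start of play, then switches it off.
; BeginPlay sets the PostProcess blend weight to full, waits StartDuration, then sets it to zero with a hard cut.
; TurnOnEffect and TurnOffEffect events perform the switching.
; A timeline-driven glitch fade-out is stubbed but unconnected, so it never runs.
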(event `self.ReceiveBeginPlay`
  (`self.TurnOnEffect`)
  (`KismetSystemLibrary.Delay` (`self.startDuration`))
  (`self.TurnOffEffect`))

(event `TurnOnEffect`
  (set `PostProcessComponent.BlendWeight` 1.0 (`self.PostProcess`)))

(event `TurnOffEffect`
  (set `PostProcessComponent.BlendWeight` 0.0 (`self.PostProcess`)))

(event `FadeOutGlitchEffect`)

(fn `UserConstructionScript`)