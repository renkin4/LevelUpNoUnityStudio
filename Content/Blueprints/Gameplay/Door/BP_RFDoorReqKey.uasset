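; Door Blueprint that opens only when the interacting character carries a key.
; CanOpenDoor casts the owner of the interactable component's current interactor to RFCharacter, then scans that character's Inventory.
; It returns true on the first item whose class derives from BP_RFPickUpKey, so any key qualifies and the check leaves it in the inventory.
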(fn `CanOpenDoor`
  (returns (ReturnValue :type Boolean))
  (bind _asrfcharacter (cast `RFCharacter` (`ActorComponent.GetOwner` (`InteractableComp.CurrentInteractor` (`self.InteractableComp`)))))
  (for _array_element (`RFCharacter.Inventory` _asrfcharacter)
    (if (`KismetMathLibrary.ClassIsChildOf` (`GameplayStatics.GetObjectClass` _array_element) "/Game/Blueprints/Gameplay/PickUp/BP_RFPickUpKey.BP_RFPickUpKey_C")
      (return true))))

(fn `UserConstructionScript`
  (`parent.UserConstructionScript`))