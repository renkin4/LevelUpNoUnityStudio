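; BP_RFWeapon is a weapon whose shot teleports the player when it hits a platform that has a teleporter attached.
; At BeginPlay it caches the first RFCharacter in the level as the player.
; ShootTrace fires a debug-drawn Visibility line trace along the given component's forward vector and spawns sparks at the hit.
; If the hit actor is a BP_RFPlatform, its attached BP_RFTeleporter teleports the cached player.
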(event `self.ReceiveBeginPlay`
  (bind _outactors (`GameplayStatics.GetAllActorsOfClass` "/Script/ProjectLvlUpGameJam.RFCharacter"))
  (set `self.player` (`|GetArrayItem` _outactors)))

(event `ShootTrace`
  (params (Start :type "CameraComponent Object Reference"))
  (bind _returnvalue (`SceneComponent.K2_GetComponentLocation` Start))
  (bind (_outhit _returnvalue_2) (`KismetSystemLibrary.LineTraceSingle` :`Start` _returnvalue :`End` (+ _returnvalue (* (`SceneComponent.GetForwardVector` Start) (`self.shootRange`))) :`TraceChannel` "TraceTypeQuery1" :`DrawDebugType` "ForDuration"))
  (if _returnvalue_2
    (bind (_bblockinghit _binitialoverlap _time _distance _location _impactpoint _normal _impactnormal _physmat _hitactor) (`GameplayStatics.BreakHitResult` _outhit))
    (`GameplayStatics.SpawnEmitterAtLocation` "/Game/ParticleSystems/PS_BulletSpark.PS_BulletSpark" _location)
    (bind _asbp_rfplatform (cast `/Game/Blueprints/Gameplay/BP_RFPlatform` _hitactor))
    (bind _asbp_rfteleporter (cast `/Game/Blueprints/Gameplay/BP_RFTeleporter` (`RFPlatform.AttachTeleporter` _asbp_rfplatform)))
    (`/Game/Blueprints/Gameplay/BP_RFTeleporter.TeleportPlayer` _asbp_rfteleporter (`self.player`))))

(fn `UserConstructionScript`)