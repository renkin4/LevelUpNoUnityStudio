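; BP_RFBullet is a projectile fired by BP_RFCharacter that teleports the shooter when it strikes a platform with an attached teleporter.
; On spawn it decrements the player's remaining shots, finding and caching the player through its instigator.
; When the projectile stops, it spawns a spark, calls TeleportPlayer on any BP_RFTeleporter attached to the hit RFPlatform, then disables collision, hides itself and expires shortly after.
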(event `self.ReceiveBeginPlay`
  ;[1 1 1] Begin Play
  (`MovementComponent.SetUpdatedComponent` (`self.ProjectileMovement`) (`self.Sphere`))
  (`/Engine/EditorBlueprintResources/StandardMacros.DecrementInt` (`/Game/Blueprints/Character/BP_RFCharacter.AmountOfShots` (`self.GetPlayer`))))

(event `DestructSelf`
  ;[1 1 1] Self Destruct
  (`PrimitiveComponent.SetCollisionEnabled` (`self.Sphere`) "NoCollision")
  (`MovementComponent.StopMovementImmediately` (`self.ProjectileMovement`))
  (`self.SetActorHiddenInGame` true)
  (`self.SetLifeSpan` 2.0))

(event `self.ProjectileMovement.OnProjectileStop`
  (params (ImpactResult :type "HitResult Structure (by ref)"))
  (bind (_bblockinghit _binitialoverlap _time _distance _location _impactpoint _normal _impactnormal _physmat _hitactor) (`GameplayStatics.BreakHitResult` ImpactResult))
  ;[1 1 1] hit events
  (`GameplayStatics.SpawnEmitterAtLocation` "/Game/ParticleSystems/PS_BulletSpark.PS_BulletSpark" _location (struct) (4.0 4.0 4.0))
  (bind _asrfplatform (cast `RFPlatform` _hitactor)
    (:`then`
      (bind _asbp_rfteleporter (cast `/Game/Blueprints/Gameplay/BP_RFTeleporter` (`RFPlatform.AttachTeleporter` _asrfplatform))
        (:`then`
          (`/Game/Blueprints/Gameplay/BP_RFTeleporter.TeleportPlayer` _asbp_rfteleporter (`self.GetPlayer`))
          (`self.DestructSelf`))
        (:`CastFailed`
          (`self.DestructSelf` :!label _label))))
    (:`CastFailed`
      (goto _label))))

(fn `GetPlayer`
  (returns (Player :type "/Game/Blueprints/Character/BP_RFCharacter Object Reference"))
  (`self.Player`
    (:`then`
      (return (`self.Player`)))
    (:`else`
      (bind _asbp_rfcharacter (cast `/Game/Blueprints/Character/BP_RFCharacter` (`self.GetInstigator`))
        (:`then`
          (set `self.Player` _asbp_rfcharacter)
          (return (`self.Player`)))
        (:`CastFailed`
          (`KismetSystemLibrary.PrintString` "FUCK SOMETHING IS WRONG DEBUG" true true (struct :`R` 1.0 :`A` 1.0) 123.0))))))

(fn `UserConstructionScript`)