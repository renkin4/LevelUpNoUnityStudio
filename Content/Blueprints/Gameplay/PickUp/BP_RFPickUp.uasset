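; BP_RFPickUp is a pickup actor that goes into the interacting RFCharacter's inventory.
; When its interactable component reports a successful interaction, it casts the interactor's owner to RFCharacter and adds itself to that character's Inventory.
; SelfDestruct then only hides the actor and disables RootBox collision, so the stored actor is never destroyed.
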(event `self.InteractableComp.InteractCompleted`
  (params (bSucceeded :type Boolean) (FailedReason :type "EFailedReason Enum" :default "FR_None"))
  ;[1 1 1] On Interaction Completed
  (if bSucceeded
    (`|ExecutionSequence`
      (:`then_0`
        (`KismetArrayLibrary.Array_Add` (`RFCharacter.Inventory` (cast `RFCharacter` (`ActorComponent.GetOwner` (`InteractableComp.CurrentInteractor` (`self.InteractableComp`))) :!pure true)) self))
      (:`then_1`
        (`self.SelfDestruct`)))))

(event `SelfDestruct`
  ;[1 1 1] Self Destruct
  (`self.SetActorHiddenInGame` true)
  (`PrimitiveComponent.SetCollisionEnabled` (`self.RootBox`) "NoCollision"))

(fn `UserConstructionScript`)