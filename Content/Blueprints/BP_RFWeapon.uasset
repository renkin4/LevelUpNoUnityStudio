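; BP_RFWeapon is a hitscan weapon that teleports the player when its shot hits a BP_RFTeleporter.
; BeginPlay caches the first RFCharacter found in the level as the player.
; ShootTrace fires a Visibility line trace along the given Start's root forward vector out to ShootRange, with debug drawing for one frame.
; A teleporter hit calls TeleportPlayer and spawns a spark emitter at the impact; other hits do nothing.
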(event `self.ReceiveBeginPlay`
  (bind _outactors (`GameplayStatics.GetAllActorsOfClass` "/Script/ProjectLvlUpGameJam.RFCharacter"))
  (set `self.player` (`|GetArrayItem` _outactors)))

(event `ShootTrace`
  (params (Start :type "CameraActor Object Reference"))
  (bind _rootcomponent (`Actor.RootComponent` Start))
  (bind _returnvalue (`SceneComponent.K2_GetComponentLocation` _rootcomponent))
  (bind (_outhit _returnvalue_2) (`KismetSystemLibrary.LineTraceSingle` :`Start` _returnvalue :`End` (+ _returnvalue (* (`SceneComponent.GetForwardVector` _rootcomponent) (`self.shootRange`))) :`TraceChannel` "TraceTypeQuery1" :`DrawDebugType` "ForOneFrame"))
  (if _returnvalue_2
    (bind (_bblockinghit _binitialoverlap _time _distance _location _impactpoint _normal _impactnormal _physmat _hitactor) (`GameplayStatics.BreakHitResult` _outhit))
    (bind _asbp_rfteleporter (cast `/Game/Blueprints/BP_RFTeleporter` _hitactor))
    (`/Game/Blueprints/BP_RFTeleporter.TeleportPlayer` _asbp_rfteleporter (`self.player`))
    (`GameplayStatics.SpawnEmitterAtLocation` "/Game/ParticleSystems/PS_BulletSpark.PS_BulletSpark" _location)))

(fn `UserConstructionScript`)