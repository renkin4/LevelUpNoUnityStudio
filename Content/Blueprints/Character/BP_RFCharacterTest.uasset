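; BP_RFCharacterTest is a test character that holds and fires a BP_RFWeapon.
; On BeginPlay it takes the first weapon found in the level and snaps it to a right-hand socket on the mesh.
; It also creates a dynamic material instance on the mesh's first slot and zeroes its Amount parameter.
; Left mouse click calls the weapon's ShootTrace, passing the follow camera.
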(event `Key|LeftMouseButton`
  (params (Key :type "Key Structure"))
  ;[1 1 1] Input
  (:`Pressed`
    (`/Game/Blueprints/Gameplay/BP_RFWeapon.ShootTrace` (`self.myWeapon`) (`self.FollowCamera`))))

(event `self.ReceiveBeginPlay`
  (bind _mesh (`self.Mesh`))
  ;[1 1 1] Begin Play
  (bind _outactors (`GameplayStatics.GetAllActorsOfClass` "/Game/Blueprints/Gameplay/BP_RFWeapon.BP_RFWeapon_C"))
  (bind _output_get (set `self.myWeapon` (`|GetArrayItem` _outactors)))
  (`SceneComponent.K2_AttachToComponent` (`Actor.RootComponent` _output_get) _mesh "RightHandIndex4" "SnapToTarget" "SnapToTarget" "KeepWorld" true)
  (bind _returnvalue (`PrimitiveComponent.CreateDynamicMaterialInstance` (`self.Mesh`) 0 (`PrimitiveComponent.GetMaterial` _mesh 0) "None"))
  (bind _output_get_2 (set `self.MaterialInstance` _returnvalue))
  (`MaterialInstanceDynamic.SetScalarParameterValue` _output_get_2 "Amount" 0.0))

(fn `UserConstructionScript`)