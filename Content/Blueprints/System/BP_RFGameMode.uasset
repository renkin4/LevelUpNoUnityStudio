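; BP_RFGameMode is a game mode that runs a repeating round countdown.
; On begin play it loads the timer from LevelRoundTime in the RF world settings and decrements it every tick.
; When time runs out, TimesUp destroys the stored player's pawn, resets the timer and destroys every BP_RFWeapon actor.
; PostLogin stores only the most recently joined PlayerController, so only that player's pawn is targeted.
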(event `self.ReceiveBeginPlay`
  ;[1 1 1] Event Begin Play
  (`parent.ReceiveBeginPlay`)
  (set `self.RoundTimer` (`KismetMathLibrary.Conv_IntToDouble` (`RFWorldSettings.LevelRoundTime` (`self.GetRFWorldSettings`)))))

(event `TimesUp`
  ;[1 1 1] Times Up
  (`self.K2_DestroyActor` (`Controller.K2_GetPawn` (`self.PlayerController`)))
  (set `self.RoundTimer` (`KismetMathLibrary.Conv_IntToDouble` (`RFWorldSettings.LevelRoundTime` (`self.GetRFWorldSettings`))))
  (bind _outactors (`GameplayStatics.GetAllActorsOfClass` "/Game/Blueprints/Gameplay/BP_RFWeapon.BP_RFWeapon_C"))
  (for _array_element _outactors
    (`self.K2_DestroyActor` _array_element)))

(event `self.ReceiveTick`
  (params (DeltaSeconds :type "Float (single-precision)"))
  ;[1 1 1] Event Tick
  (`parent.ReceiveTick` DeltaSeconds)
  (set `self.RoundTimer` (- (`self.RoundTimer`) DeltaSeconds))
  (if (<= (`self.RoundTimer`) 0.0)
    (`self.TimesUp`)))

(event `self.K2_PostLogin`
  (params (NewPlayer :type "PlayerController Object Reference"))
  ;[1 1 1] Event Post Login
  (`parent.K2_PostLogin` NewPlayer)
  (set `self.PlayerController` NewPlayer))

(fn `UserConstructionScript`)